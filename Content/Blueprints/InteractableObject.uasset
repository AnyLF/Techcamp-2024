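; InteractableObject is a Blueprint actor for an object with a mesh and a sphere collision that can be rotated.
; The construction script applies the configurable mesh to the Object component and the configurable radius to the Collision sphere.
; RotateObject adds Direction times Degree to the mesh's world roll, keeping pitch and yaw.
; The event graph holds only disabled placeholder events, so nothing in this Blueprint calls the rotation.
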(fn `RotateObject`
  (params (Direction :type Integer) (Degree :type Integer))
  (bind (_returnvalue_roll _returnvalue_pitch _returnvalue_yaw) (`KismetMathLibrary.BreakRotator` (`SceneComponent.K2_GetComponentRotation` (`self.Object`))))
  (`SceneComponent.K2_SetWorldRotation` (`self.Object`) (`KismetMathLibrary.MakeRotator` (+ (* Direction Degree) _returnvalue_roll) _returnvalue_pitch _returnvalue_yaw) false false))

(fn `UserConstructionScript`
  (`StaticMeshComponent.SetStaticMesh` (`self.Object`) (`self.Mesh`))
  (`SphereComponent.SetSphereRadius` (`self.Collision`) (`self.CollisionRadius`) true))