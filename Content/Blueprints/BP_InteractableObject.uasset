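; Base interactable object Blueprint that shows a configurable mesh, with a toggleable highlight and a rotation function.
; The construction script applies the mesh and starts with the outline off.
; ShowOutline toggles Custom Depth rendering on the mesh.
; RotateObject plays a timeline and sets world roll once per call, lerping by the stored Time toward an offset from direction, degree and acceleration.
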(fn `RotateObject`
  (params (Direction :type Integer) (Degree :type Integer) (Acceleration :type "Float (double-precision)"))
  (bind (_returnvalue_roll _returnvalue_pitch _returnvalue_yaw) (`KismetMathLibrary.BreakRotator` (`SceneComponent.K2_GetComponentRotation` (`self.Object`))))
  (`TimelineComponent.Play` (`self.RotateTimeline`))
  (`SceneComponent.K2_SetWorldRotation` (`self.Object`) (`KismetMathLibrary.MakeRotator` (`KismetMathLibrary.Lerp` _returnvalue_roll (+ (* Direction Degree Acceleration) _returnvalue_roll) (`self.Time`)) _returnvalue_pitch _returnvalue_yaw) false false))

(fn `ShowOutline`
  (params (Outline :type Boolean))
  (bind _object (`self.Object`))
  (if Outline
    (`PrimitiveComponent.SetRenderCustomDepth` _object true)
    (else
      (`PrimitiveComponent.SetRenderCustomDepth` _object false))))

(fn `UserConstructionScript`
  (`StaticMeshComponent.SetStaticMesh` (`self.Object`) (`self.Mesh`))
  (`self.ShowOutline` false))