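; BP_RotateBridge rotates a referenced static mesh actor, presumably a bridge, to a destination rotation through two player-triggered overlaps.
; Overlapping Box arms it, then overlapping the Activeate trigger plays a slowed timeline; both respond only to BP_ThirdPersonCharacter.
; Each timeline update eases in from the mesh's current rotation rather than a stored start, and disables both triggers' collision, making it one-shot.
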(event `self.activeate.OnComponentBeginOverlap`
  (params (OverlappedComponent :type "PrimitiveComponent Object Reference") (OtherActor :type "Actor Object Reference") (OtherComp :type "PrimitiveComponent Object Reference") (OtherBodyIndex :type Integer) (bFromSweep :type Boolean) (SweepResult :type "HitResult Structure (by ref)"))
  (bind _staticmesh (`self.StaticMesh`))
  (if (`self.Activated`)
    (cast `/Game/Blueprints/BP_ThirdPersonCharacter` OtherActor)
    (`TimelineComponent.SetPlayRate` (`self.Timeline`) 0.2)
    (bind (_direction _newtrack_0) (`Timeline|Timeline` :!via `PlayFromStart`)
      (:`Update`
        (`self.K2_SetActorRotation` _staticmesh (`|EaseFunction` "EaseIn" _newtrack_0 (`self.K2_GetActorRotation` _staticmesh) (`self.destinationRot`) true 2.0) false)
        (`PrimitiveComponent.SetCollisionEnabled` (`self.activeate`) "NoCollision")
        (`PrimitiveComponent.SetCollisionEnabled` (`self.Box`) "NoCollision")))))

(event `self.Box.OnComponentBeginOverlap`
  (params (OverlappedComponent :type "PrimitiveComponent Object Reference") (OtherActor :type "Actor Object Reference") (OtherComp :type "PrimitiveComponent Object Reference") (OtherBodyIndex :type Integer) (bFromSweep :type Boolean) (SweepResult :type "HitResult Structure (by ref)"))
  (cast `/Game/Blueprints/BP_ThirdPersonCharacter` OtherActor)
  (set `self.Activated` true))

(fn `UserConstructionScript`)