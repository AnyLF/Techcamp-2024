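; Holder actor that keeps collected mini lights in a spinning ring, hands them out to targets and can recall them all.
; It spawns attached holder points at BeginPlay, respaces them evenly by trigonometry as the count changes, and sends each light to its point.
; A looping timer rolls the actor to spin the ring.
; Handed-out lights and their targets are tracked, so recall returns every light and deactivates those objects.
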(event `ReTakeAllDroppedLights`
  (bind _activatedobjects (`self.ActivatedObjects`))
  (for _array_element (`self.AllDroppedLights`)
    (`KismetArrayLibrary.Array_Add` (`self.AllLightsInHolder`) _array_element))
  (`KismetArrayLibrary.Array_Clear` (`self.AllDroppedLights`))
  (`self.RelocatePoint`)
  (for (_array_element_2 _array_index) (`self.AllLightsInHolder`)
    (`/Game/Blueprints/BP_MiniLight.MoveLight` _array_element_2 (`|GetArrayItem` (`self.AllPoints`) _array_index)))
  (for _array_element_3 _activatedobjects
    (message `/Game/Blueprints/BPI_Interaction.DeactivateObject` _array_element_3))
  (`KismetArrayLibrary.Array_Clear` _activatedobjects))

(event `self.ReceiveTick`
  (params (DeltaSeconds :type "Float (single-precision)"))
  (`KismetSystemLibrary.PrintString` (`KismetStringLibrary.Concat_StrStr` "dropped: " (`KismetStringLibrary.Conv_IntToString` (`KismetArrayLibrary.Array_Length` (`self.AllDroppedLights`))) "Taken: " (`KismetStringLibrary.Conv_IntToString` (`KismetArrayLibrary.Array_Length` (`self.AllLightsInHolder`)))) true true (struct :`G` 0.66 :`B` 1.0 :`A` 1.0) DeltaSeconds))

(event `GiveOneLightFromHolder`
  (params (MoveTarget :type "Actor Object Reference"))
  (bind _alllightsinholder (`self.AllLightsInHolder`))
  (bind _output (`|GetArrayItem` _alllightsinholder (`KismetArrayLibrary.Array_LastIndex` _alllightsinholder)))
  (`self.IfNoLightInHolder`
    (:`false`
      (`/Game/Blueprints/BP_MiniLight.InstantStop` _output)
      (`KismetArrayLibrary.Array_Add` (`self.ActivatedObjects`) MoveTarget)
      (`/Game/Blueprints/BP_MiniLight.MoveLight` _output MoveTarget)
      (`KismetArrayLibrary.Array_Add` (`self.AllDroppedLights`) _output)
      (`KismetArrayLibrary.Array_RemoveItem` _alllightsinholder _output)
      (`self.RelocatePoint`)
      (`self.ReLocateAllLights`))))

(event `WhenNewLightTaken`
  (params (BP_MiniLight :type "/Game/Blueprints/BP_MiniLight Object Reference"))
  (bind _output_get (set `self.NewLight` BP_MiniLight))
  (`KismetArrayLibrary.Array_Add` (`self.AllLightsInHolder`) _output_get)
  (`self.RelocatePoint`)
  (`self.ReLocateAllLights`))

(event `ReLocateAllLights`
  (for (_array_element _array_index) (`self.AllLightsInHolder`)
    (`/Game/Blueprints/BP_MiniLight.MoveLight` _array_element (`|GetArrayItem` (`self.AllPoints`) _array_index)))
  (bind _newlight (`self.NewLight`)
    (:`then`
      (`PrimitiveComponent.SetCollisionEnabled` (`/Game/Blueprints/BP_MiniLight.Sphere` _newlight) "NoCollision")
      (`PrimitiveComponent.SetCollisionEnabled` (`/Game/Blueprints/BP_MiniLight.Sphere1` _newlight) "NoCollision"))
    (:`else`)))

(event `self.ReceiveBeginPlay`
  (`self.SpawnPoints`)
  (`self.RelocatePoint`)
  (`self.ReLocateAllLights`)
  (`KismetSystemLibrary.K2_SetTimerDelegate` (delegate `RotateAllLights`) 0.006944 true))

(event `RotateAllLights`
  (bind (_returnvalue_roll _returnvalue_pitch _returnvalue_yaw) (`KismetMathLibrary.BreakRotator` (`self.K2_GetActorRotation`)))
  (bind _result (`/Engine/EditorBlueprintResources/StandardMacros.IncrementFloat` _returnvalue_roll)
    (:`  `
      (`self.K2_SetActorRotation` (`KismetMathLibrary.MakeRotator` _result _returnvalue_pitch _returnvalue_yaw)))))

(fn `AttachAndLocateLights`
  (params (NewLocation :type "Vector Structure") (Target :type "Actor Object Reference"))
  (`self.K2_SetActorLocation` Target (+ (`self.K2_GetActorLocation`) NewLocation) false false)
  (`self.K2_AttachToActor` Target self "None" "KeepWorld" "KeepWorld" "KeepRelative" true))

(fn `RelocatePoint`
  (bind _returnvalue (`KismetArrayLibrary.Array_Length` (`self.AllLightsInHolder`)))
  (if (== _returnvalue 0)
    (`KismetSystemLibrary.PrintString` "0")
    (else
      (set `self.Angle` (/ 360 _returnvalue))
      (for _index (range _returnvalue)
        (bind _returnvalue_2 (`self.DestinationPointMaco` _index)
          (:`NewParam2`
            (`self.K2_SetActorLocation` (`|GetArrayItem` (`self.AllPoints`) _index) _returnvalue_2 false false))))))
  (return))

(fn `ResetSettingsForLightPos`
  (for _array_element (`self.AllLightsInHolder`)
    (`self.K2_DetachFromActor` _array_element "KeepRelative" "KeepRelative" "KeepRelative"))
  (return))

(fn `SpawnPoints`
  (for _index (range (`self.MaxPoint`))
    (bind _returnvalue (`|SpawnActorFromClass` "/Game/Blueprints/BP_HolderPoint.BP_HolderPoint_C" (`KismetMathLibrary.MakeTransform` (`self.K2_GetActorLocation`)) "Undefined" "MultiplyWithRoot" null _index null))
    (`KismetArrayLibrary.Array_Add` (`self.AllPoints`) _returnvalue)
    (`self.K2_AttachToActor` _returnvalue self "None" "KeepRelative" "KeepRelative" "KeepRelative" true))
  (return))

(fn `UserConstructionScript`)