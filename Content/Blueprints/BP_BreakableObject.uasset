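; BP_BreakableObject is a breakable object made of thirteen separate BETON pieces that scatter when its ObjectBreaking event is called.
; The event switches every piece to the "destructiblea" collision profile, waits briefly, then enables physics simulation on them and fires a RadialForce impulse to push them apart.
; The break is built from individual physics components, and the file does not show what triggers it.
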(event `ObjectBreaking`
  (`PrimitiveComponent.SetCollisionProfileName` (`self.BETON_02_13`) "destructiblea" true)
  (`PrimitiveComponent.SetCollisionProfileName` (`self.BETON_02_5`) "destructiblea" true)
  (`PrimitiveComponent.SetCollisionProfileName` (`self.BETON_02_4`) "destructiblea" true)
  (`PrimitiveComponent.SetCollisionProfileName` (`self.BETON_02_3`) "destructiblea" true)
  (`PrimitiveComponent.SetCollisionProfileName` (`self.BETON_02_2`) "destructiblea" true)
  (`PrimitiveComponent.SetCollisionProfileName` (`self.BETON_02_1`) "destructiblea" true)
  (`PrimitiveComponent.SetCollisionProfileName` (`self.BETON_02_6`) "destructiblea" true)
  (`PrimitiveComponent.SetCollisionProfileName` (`self.BETON_02_12`) "destructiblea" true)
  (`PrimitiveComponent.SetCollisionProfileName` (`self.BETON_02_11`) "destructiblea" true)
  (`PrimitiveComponent.SetCollisionProfileName` (`self.BETON_02_7`) "destructiblea" true)
  (`PrimitiveComponent.SetCollisionProfileName` (`self.BETON_02_10`) "destructiblea" true)
  (`PrimitiveComponent.SetCollisionProfileName` (`self.BETON_02_9`) "destructiblea" true)
  (`PrimitiveComponent.SetCollisionProfileName` (`self.BETON_02_8`) "destructiblea" true)
  (`KismetSystemLibrary.Delay` 0.01)
  (`PrimitiveComponent.SetSimulatePhysics` (`self.BETON_02_13`) true)
  (`PrimitiveComponent.SetSimulatePhysics` (`self.BETON_02_5`) true)
  (`PrimitiveComponent.SetSimulatePhysics` (`self.BETON_02_4`) true)
  (`PrimitiveComponent.SetSimulatePhysics` (`self.BETON_02_3`) true)
  (`PrimitiveComponent.SetSimulatePhysics` (`self.BETON_02_2`) true)
  (`PrimitiveComponent.SetSimulatePhysics` (`self.BETON_02_1`) true)
  (`PrimitiveComponent.SetSimulatePhysics` (`self.BETON_02_6`) true)
  (`PrimitiveComponent.SetSimulatePhysics` (`self.BETON_02_12`) true)
  (`PrimitiveComponent.SetSimulatePhysics` (`self.BETON_02_11`) true)
  (`PrimitiveComponent.SetSimulatePhysics` (`self.BETON_02_7`) true)
  (`PrimitiveComponent.SetSimulatePhysics` (`self.BETON_02_10`) true)
  (`PrimitiveComponent.SetSimulatePhysics` (`self.BETON_02_9`) true)
  (`PrimitiveComponent.SetSimulatePhysics` (`self.BETON_02_8`) true)
  (`RadialForceComponent.FireImpulse` (`self.RadialForce`)))

(fn `UserConstructionScript`)