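; BP_MiniLight is a small light actor that moves to target points and attaches to them.
; On BeginPlay it caches the light holder reference from the player's BP_ThirdPersonCharacter.
; MoveLight runs a timeline easing from its current location toward the target, then snaps and attaches; InstantStop halts that timeline.
; MoveLightToTarget uses a second timeline but leaves its parameter and ease destination unconnected.
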(event `self.ReceiveBeginPlay`
  (bind _asbp_third_person_character (cast `/Game/Blueprints/BP_ThirdPersonCharacter` (`GameplayStatics.GetPlayerPawn` 0)))
  (set `self.As BP Mini Light Holder` (`/Game/Blueprints/BP_ThirdPersonCharacter.As BP Mini Light Holder` _asbp_third_person_character)))

(event `MoveLight`
  (params (PointTarget :type "Actor Object Reference"))
  (bind (_direction _newtrack_0) (`Timeline|Timeline` :!via `PlayFromStart` :!label _label)
    (:`Update`
      (`self.K2_SetActorTransform` (`KismetMathLibrary.MakeTransform` (`|EaseFunction` "EaseIn" _newtrack_0 (`self.K2_GetActorLocation`) (`self.K2_GetActorLocation` PointTarget) 1.0))))
    (:`Finished`
      (`KismetSystemLibrary.PrintString` "Done")
      (`self.K2_AttachToActor` PointTarget "None" "SnapToTarget" "SnapToTarget" "KeepRelative"))))

(event `InstantStop`
  (goto _label :!via `Stop`))

(event `MoveLightToTarget`
  (params (NewParam :type "Vector Structure"))
  (bind (_direction _newtrack_0) (`Timeline|Timeline_0` :!via `PlayFromStart`)
    (:`Update`
      (`self.K2_SetActorTransform` (`KismetMathLibrary.MakeTransform` (`|EaseFunction` "EaseIn" _newtrack_0 (`self.K2_GetActorLocation`) (0.0 0.0 0.0) 1.0))))))

(fn `UserConstructionScript`)